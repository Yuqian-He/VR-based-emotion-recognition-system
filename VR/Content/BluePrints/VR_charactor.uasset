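; VR player character with two motion controllers for grabbing objects and moving around.
; Each grab input sends GribMessage to overlapping hand-sphere actors that implement NewInterface, keeps the last match, and sends it ReleaseMessage on release without clearing the reference.
; Left-hand axes drive movement along the left controller's forward and right vectors.
; Clicking the right controller prints a debug string and sets Speak to 1, then immediately 0.
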(event `InputAction|GrabLeft`
  (params (Key :type "Key Structure"))
  (bind _grableft (`self.GrabLeft`))
  (:`Pressed`
    (for _array_element (`PrimitiveComponent.GetOverlappingActors` (`self.SphereLeft`) null)
      (if (`KismetSystemLibrary.DoesImplementInterface` _array_element "/Game/interface/NewInterface.NewInterface_C")
        (message `/Game/interface/NewInterface.grib` _array_element (`self.MotionControllerLeft`))
        (set `self.GrabLeft` _array_element))))
  (:`Released`
    (`/Engine/EditorBlueprintResources/StandardMacros.IsValid` _grableft
      (:`Is Valid`
        (message `/Game/interface/NewInterface.release` _grableft)))))

(event `InputAction|GrabRight`
  (params (Key :type "Key Structure"))
  (bind _gribright (`self.gribRight`))
  (:`Pressed`
    (for _array_element (`PrimitiveComponent.GetOverlappingActors` (`self.SphereRight`) null)
      (if (`KismetSystemLibrary.DoesImplementInterface` _array_element "/Game/interface/NewInterface.NewInterface_C")
        (message `/Game/interface/NewInterface.grib` _array_element (`self.MotionControllerRight`))
        (set `self.gribRight` _array_element))))
  (:`Released`
    (`/Engine/EditorBlueprintResources/StandardMacros.IsValid` _gribright
      (:`Is Valid`
        (message `/Game/interface/NewInterface.release` _gribright)))))

(event `InputAxis|MovementAxisLeft_X`
  (params (AxisValue :type "Float (single-precision)"))
  (`self.AddMovementInput` (`SceneComponent.GetRightVector` (`self.MotionControllerLeft`)) AxisValue))

(event `InputAxis|MovementAxisLeft_Y`
  (params (AxisValue :type "Float (single-precision)"))
  (`self.AddMovementInput` (`SceneComponent.GetForwardVector` (`self.MotionControllerLeft`)) AxisValue))

(event `self.MotionControllerRight.OnClicked`
  (params (TouchedComponent :type "PrimitiveComponent Object Reference") (ButtonPressed :type "Key Structure"))
  (`KismetSystemLibrary.PrintString` "Hello")
  (set `self.speak` 1)
  (set `self.speak` 0))

(fn `UserConstructionScript`)