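; Small fire effect actor that drives a Niagara ground fire with configurable flames, smoke, embers and light.
; The construction script sets a fixed or seeded-random material variant, assigns the system, then pushes exposed variables into Niagara parameters, zeroing disabled ember rates and quantities.
; Optional local wind is applied at construction, while BeginPlay can instead read a level WindDirectionalSource once, setting maximum gust strength only when the minimum is positive.
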(event `self.ReceiveBeginPlay`
  (bind _niagara (`self.Niagara`))
  (bind _niagara_2 (`self.Niagara`))
  ;[1 1 1] Enable UE4 Wind Directional Source
  (if (`self.Wind Directional Source Enable`)
    (bind _returnvalue (`GameplayStatics.GetActorOfClass` "/Script/Engine.WindDirectionalSource"))
    (bind _component (`WindDirectionalSource.Component` _returnvalue))
    (bind _returnvalue_2 (`SceneComponent.GetForwardVector` _component))
    (`NiagaraComponent.SetVariableVec3` (`self.Niagara`) "User.WindDir_CF" (* _returnvalue_2 0.25))
    (`NiagaraComponent.SetVariableVec3` (`self.Niagara`) "User.WindDir" (* _returnvalue_2 (* (`WindDirectionalSourceComponent.Speed` _component) 0.75)))
    (bind _strength (`WindDirectionalSourceComponent.Strength` _component))
    (bind _returnvalue_3 (* _strength (`WindDirectionalSourceComponent.MinGustAmount` _component)))
    (if (<= _returnvalue_3 0.0)
      (`NiagaraComponent.SetVariableFloat` _niagara "User.WindStrengthMin" 0.1)
      (else
        (`NiagaraComponent.SetVariableFloat` _niagara "User.WindStrengthMin" _returnvalue_3)
        (bind _returnvalue_4 (* _strength (`WindDirectionalSourceComponent.MaxGustAmount` _component)))
        (if (<= _returnvalue_4 0.0)
          (`NiagaraComponent.SetVariableFloat` _niagara_2 "User.WindStrengthMax" 1.0)
          (else
            (`NiagaraComponent.SetVariableFloat` _niagara_2 "User.WindStrengthMax" _returnvalue_4)))))))

(fn `UserConstructionScript`
  (`|ExecutionSequence`
    (:`then_0`
      ;[1 1 1] Material Variation
      (if (`self.Use Random`)
        (set `self.Variant` (`KismetMathLibrary.RandomIntegerInRangeFromStream` 0 (- (`KismetArrayLibrary.Array_Length` (`self.Materials`)) 1) (`self.Rand`))))
      (`NiagaraComponent.SetVariableMaterial` (`self.Niagara`) "MaterialParam" (`|GetArrayItem` (`self.Materials`) (- (`self.Variant`) 1))))
    (:`then_1`
      ;[1 1 1] Set Effect
      (`NiagaraComponent.SetAsset` (`self.Niagara`) "/Game/UltimateFirePackVol1/Particles/Fire/Niagara/FireSmall/BattlefieldFire_Ground_Sm.BattlefieldFire_Ground_Sm"))
    (:`then_2`
      ;[0.439 0.7962 1 0.204] Parameters
      (`|ExecutionSequence`
        (:`then_0`
          ;;[1 1 1] Global Parameters
          (`FXSystemComponent.SetFloatParameter` (`self.Niagara`) "User.GlobalSize" (`self.Size`))
          (`FXSystemComponent.SetFloatParameter` (`self.Niagara`) "User.GlobalTurbulence" (`self.Turbulence`))
          (`FXSystemComponent.SetFloatParameter` (`self.Niagara`) "GlobalBrightness" (+ (`self.Brightness`) 1.0)))
        (:`then_1`
          ;;[1 1 1] Flames Parameters
          (`NiagaraComponent.SetVariableInt` (`self.Niagara`) "User.Speed" (`self.Speed`))
          (`FXSystemComponent.SetFloatParameter` (`self.Niagara`) "FlamesBrightnessOverdrive" (`self.Brightness Overdrive`))
          (`FXSystemComponent.SetFloatParameter` (`self.Niagara`) "FlamesTemperature" (`self.Temperature`)))
        (:`then_2`
          ;;[1 1 1] Smoke Parameters
          (`FXSystemComponent.SetFloatParameter` (`self.Niagara`) "SmokeDensity" (`self.Density`))
          (`FXSystemComponent.SetFloatParameter` (`self.Niagara`) "SmokeLifetime" (`self.Lifetime`)))
        (:`then_3`
          ;;[1 1 1] Local Wind Parameters
          (if (`self.Local Wind Enable`)
            (bind _output_get (set `self.Wind Direction` (`KismetMathLibrary.MakeVector` (`KismetMathLibrary.FClamp` (.x (`self.Wind Direction`)) -1.0) (`KismetMathLibrary.FClamp` (.y (`self.Wind Direction`)) -1.0) (`KismetMathLibrary.FClamp` (.z (`self.Wind Direction`)) -1.0))))
            (`NiagaraComponent.SetVariableVec3` (`self.Niagara`) "User.WindDir" _output_get)
            (`NiagaraComponent.SetVariableFloat` (`self.Niagara`) "WindStrengthMin" (* (`self.Wind Strength Min`) 5.0))
            (`NiagaraComponent.SetVariableFloat` (`self.Niagara`) "WindStrengthMax" (* (`self.Wind Strength Max`) 5.0))
            (`NiagaraComponent.SetVariableVec3` (`self.Niagara`) "User.WindDir_CF" (* (`self.Wind Direction`) 0.4))))
        (:`then_4`
          ;;[1 0.562 0.222 0.188] Embers Parameters
          (if (`self.Embers Enable`)
            (`|ExecutionSequence`
              (:`then_0`
                ;;;[1 1 1] Global Ember Parameters
                (`FXSystemComponent.SetFloatParameter` (`self.Niagara`) "EmbersVelocityStretch" (`self.Ember Velocity Stretch`)))
              (:`then_1`
                ;;;[1 1 1] Ambient Ember Parameters
                (if (`self.Ambient Ember Enable`)
                  (`FXSystemComponent.SetFloatParameter` (`self.Niagara`) "AmbientEmberRate" (`self.Ambient Ember Spawn Rate`))
                  (`FXSystemComponent.SetFloatParameter` (`self.Niagara`) "AmbientEmberRiseRate" (`self.Ambient Ember Rise Rate`))
                  (`FXSystemComponent.SetFloatParameter` (`self.Niagara`) "AmbientEmberTurbulenceStrength" (`self.Ambient Ember Turbulence`))
                  (`FXSystemComponent.SetFloatParameter` (`self.Niagara`) "AmbientEmberTurbulenceScale" (`self.Ambient Ember Turbulence Scale`))
                  (else
                    (`FXSystemComponent.SetFloatParameter` (`self.Niagara`) "AmbientEmberRate" 0.0))))
              (:`then_2`
                ;;;[1 1 1] Ambient Ember Intermittent Parameters
                (if (`self.Intermittent Ambient Ember Enable`)
                  (`FXSystemComponent.SetFloatParameter` (`self.Niagara`) "IntermittantAmbientEmberQuantity" (`self.Intermittent Ambient Ember Quantity`))
                  (`FXSystemComponent.SetFloatParameter` (`self.Niagara`) "IntermittantAmbientEmberIntervalMin" (`self.Intermittent Ambient Ember Interval Min`))
                  (`FXSystemComponent.SetFloatParameter` (`self.Niagara`) "IntermittantAmbientEmberIntervalMax" (`self.Intermittent Ambient Ember Interval Max`))
                  (`FXSystemComponent.SetFloatParameter` (`self.Niagara`) "IntermittantAmbientEmberRiseRate" (`self.Intermittent Ambient Ember Rise Rate`))
                  (`FXSystemComponent.SetFloatParameter` (`self.Niagara`) "IntermittantAmbientEmberTurbulenceStr" (`self.Intermittent Ambient Ember Turbulence`))
                  (`FXSystemComponent.SetFloatParameter` (`self.Niagara`) "IntermittantAmbientEmberTurbulenceScale" (`self.Intermittent Ambient Ember Turbulence Scale`))
                  (else
                    (`FXSystemComponent.SetFloatParameter` (`self.Niagara`) "IntermittantAmbientEmberQuantity" 0.0))))
              (:`then_3`
                ;;;[1 1 1] Embers Burst Parameters
                (if (`self.Ember Burst Enable`)
                  (`FXSystemComponent.SetFloatParameter` (`self.Niagara`) "EmberBurstQuantityMin" (`self.Ember Burst Quantity Min`))
                  (`FXSystemComponent.SetFloatParameter` (`self.Niagara`) "EmberBurstQuantityMax" (`self.Ember Burst Quantity Max`))
                  (`FXSystemComponent.SetFloatParameter` (`self.Niagara`) "EmberBurstIntervalMin" (`self.Ember Burst Interval Min`))
                  (`FXSystemComponent.SetFloatParameter` (`self.Niagara`) "EmberBurstIntervalMax" (`self.Ember Burst Interval Max`))
                  (`FXSystemComponent.SetFloatParameter` (`self.Niagara`) "EmberBurstInitialSpeed" (`self.Ember Burst Initial Speed`))
                  (`FXSystemComponent.SetFloatParameter` (`self.Niagara`) "EmberBurstDrag" (`self.Ember Burst Drag`))
                  (`FXSystemComponent.SetFloatParameter` (`self.Niagara`) "EmberBurstRiseRate" (`self.Ember Burst Rise Rate`))
                  (`FXSystemComponent.SetFloatParameter` (`self.Niagara`) "EmberBurstTurbulenceStrength" (`self.Ember Burst Turbulence`))
                  (`FXSystemComponent.SetFloatParameter` (`self.Niagara`) "EmberBurstTurbulenceScale" (`self.Ember Burst Turbulence Scale`))
                  (else
                    (`FXSystemComponent.SetFloatParameter` (`self.Niagara`) "EmberBurstQuantityMin" 0.0)
                    (`FXSystemComponent.SetFloatParameter` (`self.Niagara`) "EmberBurstQuantityMax" 0.0)))))
            (else
              (`FXSystemComponent.SetFloatParameter` (`self.Niagara`) "AmbientEmberRate" 0.0)
              (`FXSystemComponent.SetFloatParameter` (`self.Niagara`) "IntermittantAmbientEmberQuantity" 0.0)
              (`FXSystemComponent.SetFloatParameter` (`self.Niagara`) "EmberBurstQuantityMin" 0.0))))
        (:`then_5`
          (if (`self.Enable Light`)
            ;[1 1 1] Light Parameters
            (`FXSystemComponent.SetFloatParameter` (`self.Niagara`) "LightBrightness" (`self.Light Brightness`))
            (`FXSystemComponent.SetFloatParameter` (`self.Niagara`) "LightFlickerSpeed" (`self.Flickering Speed`))
            (`FXSystemComponent.SetFloatParameter` (`self.Niagara`) "LightRadius" (`self.Light Radius`))))))))