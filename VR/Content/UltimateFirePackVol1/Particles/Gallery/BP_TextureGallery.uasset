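; BP_TextureGallery is a display actor for a fire effect pack gallery that shows one selectable texture through a particle system.
; The construction script applies the exposed Material to the PSTextureDisplay component and passes TextureSelect as a float particle parameter, so the choice previews in the editor.
; BeginPlay reapplies only the material when the game starts.
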(event `self.ReceiveBeginPlay`
  (`PrimitiveComponent.SetMaterial` (`self.PS_TextureDisplay`) 0 (`self.Material`)))

(fn `UserConstructionScript`
  (`PrimitiveComponent.SetMaterial` (`self.PS_TextureDisplay`) 0 (`self.Material`))
  (`FXSystemComponent.SetFloatParameter` (`self.PS_TextureDisplay`) "TextureSelect" (`KismetMathLibrary.Conv_IntToDouble` (`self.TextureSelect`))))