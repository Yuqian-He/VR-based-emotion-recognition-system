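; BP_Fireworks is a Blueprint actor that fires a fireworks effect when its Trigger event is called.
; Trigger optionally activates the Launch effect component if UseLaunchFx is set, then spawns the NSFxFireworks system at the root component's world location.
; The construction script places Launch at the root location plus LaunchFxOffset, so the launch effect can be offset separately from the burst.
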(event `Trigger`
  (if (`self.UseLaunchFx`)
    (`ActorComponent.Activate` (`self.Launch`) false))
  (`NiagaraFunctionLibrary.SpawnSystemAtLocation` (`self.NS_Fx_Fireworks`) (`SceneComponent.K2_GetComponentLocation` (`self.DefaultSceneRoot`))))

(fn `UserConstructionScript`
  (`SceneComponent.K2_SetWorldLocation` (`self.Launch`) (+ (`SceneComponent.K2_GetComponentLocation` (`self.DefaultSceneRoot`)) (`self.LaunchFxOffset`)) false false))