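; Fireworks actor that, on Trigger, launches a timed sequence of Niagara fireworks from its root location.
; Trigger loops through the NSFxFireworks array with a LaunchInterval delay between spawns, resetting the index after the last.
; Before each spawn, SetBoomPosition randomizes burst XY and height, which pass to Niagara variables; it also computes LaunchDirection, unused in these graphs.
; The construction script positions the Launch component at LaunchFxOffset from the root.
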(event `Trigger`
  (`self.SetBoomPosition` :!label _label)
  (bind _returnvalue (`NiagaraFunctionLibrary.SpawnSystemAtLocation` (`|GetArrayItem` (`self.NS_Fx_Fireworks`) (`self.CurrentIndex`)) (`SceneComponent.K2_GetComponentLocation` (`self.DefaultSceneRoot`))))
  (`NiagaraComponent.SetVariableFloat` _returnvalue "BoomPositionX" (`self.BoomPositionX`))
  (`NiagaraComponent.SetVariableFloat` _returnvalue "BoomPositionY" (`self.BoomPositionY`))
  (`NiagaraComponent.SetVariableFloat` _returnvalue "Height" (`self.Height`))
  (bind _output_get (set `self.CurrentIndex` (+ (`self.CurrentIndex`) 1)))
  (`KismetSystemLibrary.Delay` (`self.LaunchInterval`))
  (if (< _output_get (`KismetArrayLibrary.Array_Length` (`self.NS_Fx_Fireworks`)))
    (goto _label)
    (else
      (set `self.CurrentIndex` 0))))

(fn `SetBoomPosition`
  (bind _output_get (set `self.BoomPositionX` (* (- (* (`KismetMathLibrary.RandomFloat`) 2.0) 1.0) (`self.RangeScale_XY`))))
  (bind _output_get_2 (set `self.BoomPositionY` (* (- (* (`KismetMathLibrary.RandomFloat`) 2.0) 1.0) (`self.RangeScale_XY`))))
  (bind _output_get_3 (set `self.Height` (+ (* (- (* (`KismetMathLibrary.RandomFloat`) 2.0) 1.0) 500.0) (`self.DefaultHeight`))))
  (set `self.LaunchDirection` (`KismetMathLibrary.Normal` (`KismetMathLibrary.MakeVector` _output_get _output_get_2 _output_get_3))))

(fn `UserConstructionScript`
  (`SceneComponent.K2_SetWorldLocation` (`self.Launch`) (+ (`SceneComponent.K2_GetComponentLocation` (`self.DefaultSceneRoot`)) (`self.LaunchFxOffset`)) false false))